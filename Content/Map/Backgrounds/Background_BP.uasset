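; Background_BP is a background actor that shifts along X in response to the player's horizontal movement, apparently for a parallax effect.
; Each Tick casts the Player reference to Player_BP, checks the sign of its X velocity and builds an X-only offset from velocity magnitude times Speed.
; Negative velocity adds that offset to the actor's location, while positive velocity divides the location by it rather than subtracting, before setting relative location.
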(event EventBeginPlay)

(event Collision|EventActorBeginOverlap
  (params (OtherActor :type Actor%20Object%20Reference)))

(event EventTick
  (params (DeltaSeconds :type Float%20%28single-precision%29))
  (bind _returnvalue (Transformation|GetActorLocation))
  (bind _asplayer_bp (Utilities|Casting|CastToPlayer_BP (Variables|Default|GetPlayer)))
  (Math|Float|CompareFloat (.X (Math|Vector|BreakVector (Variables|/Script/Engine.MovementComponent|GetVelocity (Variables|/Script/Engine.Character|GetCharacterMovement _asplayer_bp)))) 0.0
    (:>
      (Transformation|SetActorRelativeLocation (/ _returnvalue (Math|Vector|MakeVector (* (Math|Vector|VectorLength (Variables|/Script/Engine.MovementComponent|GetVelocity (Variables|/Script/Engine.Character|GetCharacterMovement _asplayer_bp))) (Variables|Default|GetSpeed)) 0.0 0.0))))
    (:<
      (Transformation|SetActorRelativeLocation (+ (Math|Vector|MakeVector (* (Math|Vector|VectorLength (Variables|/Script/Engine.MovementComponent|GetVelocity (Variables|/Script/Engine.Character|GetCharacterMovement _asplayer_bp))) (Variables|Default|GetSpeed)) 0.0 0.0) _returnvalue)))))

(fn ConstructionScript)