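; Side-scrolling camera actor that becomes the view target, follows the player and drives a parallax sky background.
; On BeginPlay it converts its X clamp to world space, creates the background's dynamic material and teleports to the player.
; Each tick it accumulates a material scroll offset at fixed speed based on horizontal movement and direction.
; It then interpolates toward the player's clamped X, following Z only when FollowZAxis is set.
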(event Custom|UpdateCameraPosition
  (bind _playerref (Variables|Default|GetPlayerRef))
  (bind _leftxaxismin (Variables|Default|GetLeftXAxisMin))
  (bind _rightxaxismax (Variables|Default|GetRightXAxisMax))
  (bind _returnvalue (Transformation|GetActorLocation _playerref))
  (bind _returnvalue_2 (Math|Float|Clamp(Float) (.x _returnvalue) _leftxaxismin _rightxaxismax))
  (Utilities|IsValid _playerref
    (:Is%20Valid
      (if (Variables|Default|GetFollowZAxis)
        (Transformation|SetActorLocation (Math|Interpolation|VInterpTo (Transformation|GetActorLocation) (Math|Vector|MakeVector _returnvalue_2 0.0 (.z _returnvalue)) (Utilities|Time|GetWorldDeltaSeconds) 2e+01) false false)
        (else
          (Transformation|SetActorLocation (Math|Interpolation|VInterpTo (Transformation|GetActorLocation) (Math|Vector|MakeVector _returnvalue_2 0.0 (.z (Transformation|GetActorLocation))) (Utilities|Time|GetWorldDeltaSeconds) 2e+01) false false))))))

(event EventBeginPlay
  (bind _returnvalue (Transformation|GetActorTransform))
  (bind _cameraxaxisclamp (Variables|Default|GetCameraXAxisClamp))
  (bind _asplayer_bp (Utilities|Casting|CastToPlayer_BP (Game|GetPlayerCharacter 0)))
  (Variables|Default|SetPlayerRef _asplayer_bp)
  (Variables|Default|SetLeftXAxisMin (.x (Math|Transform|TransformLocation _returnvalue (Utilities|Array|Get(acopy) _cameraxaxisclamp))))
  (Variables|Default|SetRightXAxisMax (.x (Math|Transform|TransformLocation _returnvalue (Utilities|Array|Get(acopy) _cameraxaxisclamp 1))))
  (Utilities|IsValid (Variables|Default|GetPlayerRef)
    (:Is%20Valid
      (bind _returnvalue_2 (Rendering|Material|CreateDynamicMaterialInstance (Variables|Default|GetBackground) 0 "/Game/Backgrounds/SkyParallax.SkyParallax" "None" :!class /Script/Engine.PrimitiveComponent))
      (Variables|Default|SetMID _returnvalue_2)
      (Game|Player|SetViewTargetwithBlend (Game|GetPlayerController 0) self 0.0 "VTBlend_Linear" 0.0 false)
      (Transformation|Teleport (+ (Variables|Default|GetOffset) (Math|Vector|MakeVector (.x (Transformation|GetActorLocation (Variables|Default|GetPlayerRef))) 0.0 (.z (Transformation|GetActorLocation (Variables|Default|GetPlayerRef))))) (Transformation|GetActorRotation)))))

(event EventTick
  (params (DeltaSeconds :type Float%20%28single-precision%29))
  (Utilities|IsValid (Variables|Default|GetPlayerRef)
    (:Is%20Valid
      (Variables|Default|SetDelta (* (Utilities|Time|GetWorldDeltaSeconds) (Math|Vector|VectorLength (* (Class|KismetMathLibrary|VectorNormal2D (Math|Vector|MakeVector (.x (Transformation|GetVelocity (Variables|Default|GetPlayerRef))) 0.0 0.0) 0.0001) (Variables|Default|GetBackground_Speed)))))
      (bind _movingright (Default|GetMovingRight (Variables|Default|GetPlayerRef)))
      (if _movingright
        _
        (else
          (bind _result (Math|Float|NegateFloat (Variables|Default|GetDelta))
            (:%20%20
              (Variables|Default|SetDelta _result)))))
      (Variables|Default|SetCurrentOffset (+ (Variables|Default|GetCurrentOffset) (Variables|Default|GetDelta)))
      (if (> (Variables|Default|GetCurrentOffset) 1.0)
        (Variables|Default|SetCurrentOffset (.Remainder (Math|Float|Division(WholeandRemainder) (Variables|Default|GetCurrentOffset) 1.0))))
      (Rendering|Material|SetScalarParameterValue (Variables|Default|GetMID) "Offset" (Variables|Default|GetCurrentOffset) :!class /Script/Engine.MaterialInstanceDynamic)
      (CallFunction|UpdateCameraPosition))))

(fn ConstructionScript)