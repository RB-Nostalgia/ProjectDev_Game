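; Player character for a 2D flipbook side-scroller with walk, run, jump, attack, damage and pause menu.
; Tick picks movement or death flipbooks through FlipbookFunction's state-to-asset select and flips control rotation by X velocity.
; Attacks lock input for the flipbook's length, then apply damage through a short pawn line trace.
; Incoming damage lowers Health, updates the heart HUD icon and shows the damaged flipbook.
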(event Custom|UpdateControlRotation
  ;[1 1 1] Rotate Char
  (Utilities|IsValid (Pawn|GetController)
    (:Is%20Valid
      (Math|Float|CompareFloat (.X (Math|Vector|BreakVector (Variables|/Script/Engine.MovementComponent|GetVelocity (Variables|Character|GetCharacterMovement)))) 0.0
        (:>
          (Pawn|SetControlRotation (Pawn|GetController) (Math|Rotator|MakeRotator 0.0 0.0 0.0)))
        (:<
          (Pawn|SetControlRotation (Pawn|GetController) (Math|Rotator|MakeRotator 0.0 0.0 1.8e+02)))))))

(event Custom|Change_Icon
  (params (Health :type Float%20%28double-precision%29))
  ;[1 1 1] Health Stuff
  (if (== Health 4.0)
    (bind _output_get (Variables|Default|SetHealth%20Icon%20Def (Variables|Default|GetHealth_Icon_1)))
    (Default|GetIcon (Variables|Default|GetHealth%20UI%20Ref) _output_get)
    (elif (== Health 3.0)
      (bind _output_get_2 (Variables|Default|SetHealth%20Icon%20Def (Variables|Default|GetHealth_Icon_2)))
      (Default|GetIcon (Variables|Default|GetHealth%20UI%20Ref) _output_get_2)
      (elif (== Health 2.0)
        (bind _output_get_3 (Variables|Default|SetHealth%20Icon%20Def (Variables|Default|GetHealth_Icon_3)))
        (Default|GetIcon (Variables|Default|GetHealth%20UI%20Ref) _output_get_3)
        (elif (== Health 1.0)
          (bind _output_get_4 (Variables|Default|SetHealth%20Icon%20Def (Variables|Default|GetHealth_Icon_4)))
          (Default|GetIcon (Variables|Default|GetHealth%20UI%20Ref) _output_get_4)
          (elif (== Health 0.0)
            (bind _output_get_5 (Variables|Default|SetHealth%20Icon%20Def (Variables|Default|GetHealth_Icon_5)))
            (Default|GetIcon (Variables|Default|GetHealth%20UI%20Ref) _output_get_5)))))))

(event Custom|Update%20Animation
  ;[1 1 1] Moving
  (if (not (AI|Components|NavMovement|IsFalling (Variables|Character|GetCharacterMovement)))
    (if (> (Variables|Default|GetHealth) 0.0)
      (if (Variables|Default|GetIsAttacking)
        (CallFunction|FlipbookFunction "NewEnumerator3")
        (elif (Variables|Default|GetIsRunning)
          (CallFunction|FlipbookFunction "NewEnumerator5")
          (else
            (CallFunction|FlipbookFunction (select (> (Math|Vector|VectorLength (Transformation|GetVelocity)) 0.0) "NewEnumerator1" "NewEnumerator0")))))
      (else
        (CallFunction|FlipbookFunction "NewEnumerator4")
        (Pawn|Components|CharacterMovement|DisableMovement (Variables|Character|GetCharacterMovement))
        (Utilities|FlowControl|Delay (Class|PaperFlipbookComponent|GetFlipbookLength (Variables|Default|GetSprite)))
        (Audio|Components|Audio|Stop (Variables|Default|GetSprite))))))

(event EventBeginPlay
  ;[1 1 1] HUD Creation
  (Variables|/Script/Engine.CharacterMovementComponent|SetMaxWalkSpeed (Variables|Character|GetCharacterMovement) (Variables|Default|GetWalkSpeed))
  (bind _returnvalue (UserInterface|CreateWidget "/Game/Blueprints/Blueprints_UI/HUD_Heart.HUD_Heart_C"))
  (bind _output_get (Variables|Default|SetHealth%20UI%20Ref _returnvalue))
  (UserInterface|Viewport|AddtoViewport _output_get 0))

(event Game|Damage|EventAnyDamage
  (params (Damage :type Float%20%28single-precision%29) (DamageType :type Damage%20Type%20Object%20Reference) (InstigatedBy :type Controller%20Object%20Reference) (DamageCauser :type Actor%20Object%20Reference))
  ;[1 1 1] On Take Damage
  (if (!= (Variables|Default|GetIsDead) true)
    (Variables|Default|SetHealth (- (Variables|Default|GetHealth) Damage))
    (CallFunction|ChangeIcon (Variables|Default|GetHealth))
    (CallFunction|FlipbookFunction "NewEnumerator6")))

(event EventTick
  (params (DeltaSeconds :type Float%20%28single-precision%29))
  ;[1 1 1] Moving
  (if (not (Variables|Default|GetIsAttacking))
    (CallFunction|UpdateAnimation)
    (CallFunction|UpdateControlRotation)))

(event Input|ActionEvents|InputActionJump
  (params (Key :type Key%20Structure :default "None"))
  ;[1 1 1] Jumping
  (:Pressed
    (Character|Jump)
    (CallFunction|FlipbookFunction "NewEnumerator2")
    (Utilities|FlowControl|Delay (Class|PaperFlipbookComponent|GetFlipbookLength (Variables|Default|GetSprite))))
  (:Released
    (Character|StopJumping)))

(event Input|ActionEvents|InputActionAttack
  (params (Key :type Key%20Structure :default "None"))
  (bind _returnvalue (Transformation|GetActorLocation))
  ;[1 1 1] Attacking
  (:Pressed
    (Variables|Default|SetIsAttacking true)
    (if (>= (Variables|Default|GetHealth) 1.0)
      (CallFunction|FlipbookFunction "NewEnumerator3")
      (Input|DisableInput 0)
      (Utilities|FlowControl|Delay (Class|PaperFlipbookComponent|GetFlipbookLength (Variables|Default|GetSprite)))
      (Utilities|FlowControl|Sequence
        (:then_0
          (Variables|Default|SetIsAttacking false)
          (Input|EnableInput 0))
        (:then_1
          (bind _outhit (Collision|LineTraceForObjects _returnvalue (+ _returnvalue (* (Transformation|GetActorForwardVector) (Math|Vector|MakeVector 4e+01 0.0 0.0))) (Utilities|Array|MakeArray "ObjectTypeQuery3") false (Utilities|Array|MakeArray self) "None"))
          (if (not (== (Game|GetPlayerCharacter 0) (.HitActor (Collision|BreakHitResult _outhit))))
            (Game|Damage|ApplyDamage (.HitActor (Collision|BreakHitResult _outhit)) (Variables|Default|GetDamage) 0 self))))))
  (:Released
    (Variables|Default|SetIsAttacking false)))

(event Input|ActionEvents|InputActionPause
  (params (Key :type Key%20Structure :default "None"))
  (bind _returnvalue (Game|GetPlayerController 0))
  (bind _returnvalue_2 (Game|GetPlayerController 0))
  (:Pressed
    (Utilities|FlowControl|FlipFlop
      (:A
        (bind _returnvalue_3 (UserInterface|CreateWidget "/Game/MenuButton/PauseMenu.PauseMenu_C"))
        (UserInterface|Viewport|AddtoViewport _returnvalue_3 0)
        (Game|SetGamePaused true)
        (Input|SetInputModeGameandUI _returnvalue 0 "DoNotLock" true false)
        (Variables|/Script/Engine.PlayerController|SetbShowMouseCursor _returnvalue true))
      (:B
        (Widget|RemovefromParent _returnvalue_3)
        (Input|SetInputModeGameOnly _returnvalue_2 false)
        (Variables|/Script/Engine.PlayerController|SetbShowMouseCursor _returnvalue_2 false)
        (Game|SetGamePaused false)))))

(event Input|ActionEvents|InputActionRun
  (params (Key :type Key%20Structure :default "None"))
  ;[1 1 1] Running
  (:Pressed
    (if (> (Variables|Default|GetHealth) 0.0)
      (Variables|Default|SetIsRunning true)
      (Variables|/Script/Engine.CharacterMovementComponent|SetMaxWalkSpeed (Variables|Character|GetCharacterMovement) (Variables|Default|GetRunSpeed))))
  (:Released
    (Variables|Default|SetIsRunning false)
    (Variables|/Script/Engine.CharacterMovementComponent|SetMaxWalkSpeed (Variables|Character|GetCharacterMovement) (Variables|Default|GetWalkSpeed))))

(event Input|AxisEvents|InputAxisMoveRight
  (params (AxisValue :type Float%20%28single-precision%29))
  ;[1 1 1] Moving
  (Pawn|Input|AddMovementInput "1.000000,0.000000,0.000000" AxisValue false))

(fn ConstructionScript)

(fn FlipbookFunction
  (params (Current_State :type Animation_States%20Enum :default "NewEnumerator0"))
  (Variables|Default|SetAnim_States Current_State)
  (Sprite|SetFlipbook (Variables|Default|GetSprite) (Utilities|Select :Index (Variables|Default|GetAnim_States) :NewEnumerator3 (Variables|Default|GetAttack_FB) :NewEnumerator0 (Variables|Default|GetIdle_FB%20) :NewEnumerator1 (Variables|Default|GetWalk_FB) :NewEnumerator2 (Variables|Default|GetJump_FB) :NewEnumerator4 (Variables|Default|GetDeath_FB) :NewEnumerator5 (Variables|Default|GetRun_FB) :NewEnumerator6 (Variables|Default|GetDamaged_FB)))
  (return))