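; Skeleton_BP is a flipbook-animated patrolling melee enemy, using Mushroom flipbooks, that damages the player and can be killed.
; Tick drives animation and movement, with a forward line trace triggering a pause and turnaround.
; Hitbox overlap starts a looping timer that plays the attack, then box-traces to apply damage, gated by DoOnce cooldown.
; Incoming damage triggers a hit reaction and attack-blocking stun, or death and destruction; knockback logic is unconnected.
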(event OnComponentBeginOverlap(Hitbox)
  (params (OverlappedComponent :type Primitive%20Component%20Object%20Reference) (OtherActor :type Actor%20Object%20Reference) (OtherComp :type Primitive%20Component%20Object%20Reference) (OtherBodyIndex :type Integer) (bFromSweep :type Boolean) (SweepResult :type Hit%20Result%20Structure%20%28by%20ref%29))
  ;[1 1 1] Enemy Attack
  (bind _asplayer_bp (Utilities|Casting|CastToPlayer_BP OtherActor))
  (bind _returnvalue (Utilities|Time|SetTimerbyEvent (delegate Custom|Attack%20Player) 1.0 true))
  (Variables|Default|SetAttack_Event _returnvalue))

(event OnComponentEndOverlap(Hitbox)
  (params (OverlappedComponent :type Primitive%20Component%20Object%20Reference) (OtherActor :type Actor%20Object%20Reference) (OtherComp :type Primitive%20Component%20Object%20Reference) (OtherBodyIndex :type Integer))
  (bind _returnvalue (Transformation|GetActorLocation))
  ;[1 1 1] Enemy Attack
  (Utilities|Casting|CastToPlayer_BP OtherActor)
  (Utilities|Time|ClearandInvalidateTimerbyHandle (Variables|Default|GetAttack_Event))
  (Utilities|FlowControl|DoOnce false) ; enters at Reset
)

(event Custom|AnimationUpdate
  ;[1 1 1] Animation Update
  (if (Variables|Default|GetBeingAttacked)
    (Sprite|SetFlipbook (Variables|Default|GetSprite) (Variables|Default|GetMushroom_Take%20Damage))
    (else
      (Sprite|SetFlipbook (Variables|Default|GetSprite) (select (> (Math|Vector|VectorLength (Variables|/Script/Engine.MovementComponent|GetVelocity (Variables|Character|GetCharacterMovement))) 0.0) (Variables|Default|GetMushroom_Run_FB) (Variables|Default|GetMushroom_Idle_FB))))))

(event Custom|MovementUpdate
  (bind _returnvalue (Transformation|GetActorLocation))
  ;[1 1 1] Movement Update
  (if (not (Variables|Default|GetBeingAttacked))
    (Utilities|FlowControl|Sequence
      (:then_0
        (if (> (Variables|Default|GetMovement_Direction) 0.0)
          (Transformation|SetActorRotation "0, 0, 0")
          (else
            (Transformation|SetActorRotation "0.000000,180.000000,0.000000"))))
      (:then_1
        (Pawn|Input|AddMovementInput "1.000000,0.000000,0.000000" (Variables|Default|GetMovement_Direction) false)
        (bind _returnvalue_2 (Collision|LineTraceByChannel _returnvalue (+ (* (Transformation|GetActorForwardVector) (Math|Vector|MakeVector 20.5 0.0 0.0)) _returnvalue) "TraceTypeQuery1" false 0 "None"))
        (if _returnvalue_2
          (Utilities|FlowControl|DoOnce false :!label _label
            (:Completed
              (Variables|/Script/Engine.CharacterMovementComponent|SetMaxWalkSpeed (Variables|Character|GetCharacterMovement) 0.0)
              (Utilities|FlowControl|Delay (Variables|Default|GetDuration))
              (Variables|/Script/Engine.CharacterMovementComponent|SetMaxWalkSpeed (Variables|Character|GetCharacterMovement) (Variables|Default|GetMax%20Walk%20Speed))
              (Variables|Default|SetMovement_Direction (* (Variables|Default|GetMovement_Direction) -1.0))
              (goto _label Reset))))))))

(event Custom|Attack%20Player
  (bind _returnvalue (Transformation|GetActorLocation))
  ;[1 1 1] Enemy Attack
  (if (not (Variables|Default|GetIsDead))
    (if (not (Variables|Default|GetBeingAttacked))
      (if (> (Variables|/Game/Blueprints/Blueprints_Player/Player_BP.Player_BP_C|GetHealth (stale OnComponentBeginOverlap(Hitbox) _asplayer_bp)) 0.0)
        (if (not (Variables|Default|GetisStunned))
          (Utilities|FlowControl|DoOnce false :!label _label
            (:Completed
              (Variables|Default|SetIsAttacking true)
              (Utilities|FlowControl|Delay (Class|PaperFlipbook|GetTotalDuration (Variables|Default|GetMushroom_Damage_FB)))
              (Utilities|FlowControl|Sequence
                (:then_0
                  (Variables|Default|SetIsAttacking false))
                (:then_1
                  (bind _outhit (Class|KismetSystemLibrary|BoxTraceSingleforObjects _returnvalue (+ _returnvalue (* (Transformation|GetActorForwardVector) (Math|Vector|MakeVector 3e+01 0.0 0.0))) "20.000000,20.000000,20.000000" "0, 0, 0" (Utilities|Array|MakeArray "ObjectTypeQuery3") false (Utilities|Array|MakeArray self) "None" true "(R=1.000000,G=0.000000,B=0.000000,A=1.000000)" "(R=0.000000,G=1.000000,B=0.000000,A=1.000000)" 0.2))
                  (if (== (Game|GetPlayerCharacter 0) (.HitActor (Collision|BreakHitResult _outhit)))
                    (Game|Damage|ApplyDamage (.HitActor (Collision|BreakHitResult _outhit)) (Variables|Default|GetEnemyDamage) 0 self)
                    (Utilities|FlowControl|Delay (Variables|Default|GetAttack_CD))
                    (goto _label Reset)))))))))))

(event EventBeginPlay
  (Variables|/Script/Engine.CharacterMovementComponent|SetMaxWalkSpeed (Variables|Character|GetCharacterMovement) (Variables|Default|GetMax%20Walk%20Speed)))

(event Game|Damage|EventAnyDamage
  (params (Damage :type Float%20%28single-precision%29) (DamageType :type Damage%20Type%20Object%20Reference) (InstigatedBy :type Controller%20Object%20Reference) (DamageCauser :type Actor%20Object%20Reference))
  (bind _mushroom_take_damage (Variables|Default|GetMushroom_Take%20Damage))
  ;[1 1 1] On Take Damage
  (Variables|Default|SetSlime_Health (- (Variables|Default|GetSlime_Health) Damage))
  (if (<= (Variables|Default|GetSlime_Health) 0.0)
    (Variables|Default|SetIsDead true)
    (Sprite|SetFlipbook (Variables|Default|GetSprite) (Variables|Default|GetMushroom_Dead_FB))
    (Components|DestroyComponent (Variables|Default|GetCapsuleComponent))
    (Utilities|FlowControl|Delay (Class|PaperFlipbook|GetTotalDuration (Variables|Default|GetMushroom_Dead_FB)))
    (Audio|Components|Audio|Stop (Variables|Default|GetSprite))
    (Utilities|FlowControl|Delay 0.5)
    (Actor|DestroyActor)
    (elif (not (Variables|Default|GetBeingAttacked))
      (Variables|Default|SetBeingAttacked true)
      (Variables|Default|SetisStunned true)
      (Sprite|SetFlipbook (Variables|Default|GetSprite) _mushroom_take_damage)
      (Utilities|FlowControl|Delay (Class|PaperFlipbook|GetTotalDuration _mushroom_take_damage))
      (Variables|Default|SetBeingAttacked false)
      (Utilities|FlowControl|Delay (Variables|Default|GetStun_Duration))
      (Variables|Default|SetisStunned false))))

(event EventTick
  (params (DeltaSeconds :type Float%20%28single-precision%29))
  (if (not (Variables|Default|GetIsDead))
    (if (Variables|Default|GetIsAttacking)
      (Sprite|SetFlipbook (Variables|Default|GetSprite) (Variables|Default|GetMushroom_Damage_FB))
      (Utilities|FlowControl|Delay (Class|PaperFlipbook|GetTotalDuration (Variables|Default|GetMushroom_Damage_FB)))
      (Variables|Default|SetIsAttacking false)
      (else
        (CallFunction|AnimationUpdate)
        (CallFunction|MovementUpdate)))))

(fn ConstructionScript)